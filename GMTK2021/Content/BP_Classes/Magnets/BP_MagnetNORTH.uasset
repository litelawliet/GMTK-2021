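; North-pole magnet actor that attracts other magnets attached to different objects.
; Each Tick, ApplyInfluence scans ActionRange overlaps for BP_MagnetBase actors, requiring both Spheres to simulate physics.
; The attached objects' EMovableType decides which Sphere gets pulled: walls stay put, small boxes move toward big ones, equal boxes attract mutually.
; Force falls off quadratically with distance, using MaxAttractForce as both strength and cutoff; MaxDistance is unused.
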(event EventTick
  (params (DeltaSeconds :type Float%20%28single-precision%29))
  (CallFunction|ApplyInfluence (Variables|Default|GetSphere) (Variables|Default|GetActionRange) (Components|Sphere|GetScaledSphereRadius (Variables|Default|GetActionRange))))

(event EventBeginPlay
  (|CallParentFunction))

(fn ConstructionScript
  (|CallParentFunction))

(fn ApplyInfluence
  (params (Pole :type Primitive%20Component%20Object%20Reference%20%28by%20ref%29) (ActionRange :type Primitive%20Component%20Object%20Reference%20%28by%20ref%29) (MaxDistance :type Float%20%28single-precision%29))
  (bind _maxattractforce (Variables|Default|GetMaxAttractForce))
  (bind _attachedobject (Variables|Default|GetAttachedObject))
  (bind _emovabletype (Variables|/Game/BP_Classes/SurfaceTypes/BP_ShootableBase.BP_ShootableBase_C|GeteMovableType _attachedobject))
  (LocalVariables|SetL_Pole Pole)
  (LocalVariables|SetL_ActionRange ActionRange)
  (LocalVariables|SetL_MaxDistance MaxDistance)
  (for _array_element (Class|PrimitiveComponent|GetOverlappingComponents (LocalVariables|GetL_ActionRange))
    (bind _output_get (LocalVariables|SetL_Foreign_Pole _array_element))
    (if (!= _output_get (LocalVariables|GetL_Pole))
      (bind _asbp_magnet_base (Utilities|Casting|CastToBP_MagnetBase (Components|GetOwner (LocalVariables|GetL_Foreign_Pole))))
      (if (and (Utilities|IsValid (Variables|/Game/BP_Classes/Magnets/BP_MagnetBase.BP_MagnetBase_C|GetAttachedObject _asbp_magnet_base)) (Utilities|IsValid _attachedobject))
        (if (!= _attachedobject (Variables|/Game/BP_Classes/Magnets/BP_MagnetBase.BP_MagnetBase_C|GetAttachedObject _asbp_magnet_base))
          (if (and (Physics|IsSimulatingPhysics (Variables|/Game/BP_Classes/Magnets/BP_MagnetBase.BP_MagnetBase_C|GetSphere _asbp_magnet_base) "None") (Physics|IsSimulatingPhysics (Variables|Default|GetSphere) "None"))
            (switch int (Variables|/Game/BP_Classes/SurfaceTypes/BP_ShootableBase.BP_ShootableBase_C|GeteMovableType (Variables|/Game/BP_Classes/Magnets/BP_MagnetBase.BP_MagnetBase_C|GetAttachedObject _asbp_magnet_base))
              (:0
                ;[1 1 1] South is Wall => all except North wall gets addforced
                (if (!= _emovabletype 0)
                  (Physics|AddForce (Variables|Default|GetSphere) (* (* (Math|Vector|Normalize (- (Physics|GetCenterOfMass (LocalVariables|GetL_Pole) "None") (Physics|GetCenterOfMass (LocalVariables|GetL_Foreign_Pole) "None"))) (* (Math|Float|Square (/ (- _maxattractforce (Math|Float|Clamp(Float) (Math|Vector|VectorLength (- (Physics|GetCenterOfMass (LocalVariables|GetL_Pole) "None") (Physics|GetCenterOfMass (LocalVariables|GetL_Foreign_Pole) "None"))) 0.0 _maxattractforce)) _maxattractforce)) _maxattractforce)) -1.0) "None" false)))
              (:1
                ;[1 1 1] South is small box
                (switch int _emovabletype
                  (:0
                    (Physics|AddForce (Variables|/Game/BP_Classes/Magnets/BP_MagnetBase.BP_MagnetBase_C|GetSphere _asbp_magnet_base) (* (Math|Vector|Normalize (- (Physics|GetCenterOfMass (LocalVariables|GetL_Pole) "None") (Physics|GetCenterOfMass (LocalVariables|GetL_Foreign_Pole) "None"))) (* (Math|Float|Square (/ (- _maxattractforce (Math|Float|Clamp(Float) (Math|Vector|VectorLength (- (Physics|GetCenterOfMass (LocalVariables|GetL_Pole) "None") (Physics|GetCenterOfMass (LocalVariables|GetL_Foreign_Pole) "None"))) 0.0 _maxattractforce)) _maxattractforce)) _maxattractforce)) "None" false :!label _label))
                  (:1
                    (Physics|AddForce (Variables|Default|GetSphere) (* (* (Math|Vector|Normalize (- (Physics|GetCenterOfMass (LocalVariables|GetL_Pole) "None") (Physics|GetCenterOfMass (LocalVariables|GetL_Foreign_Pole) "None"))) (* (Math|Float|Square (/ (- _maxattractforce (Math|Float|Clamp(Float) (Math|Vector|VectorLength (- (Physics|GetCenterOfMass (LocalVariables|GetL_Pole) "None") (Physics|GetCenterOfMass (LocalVariables|GetL_Foreign_Pole) "None"))) 0.0 _maxattractforce)) _maxattractforce)) _maxattractforce)) -1.0) "None" false)
                    (goto _label))
                  (:2
                    (Physics|AddForce (Variables|/Game/BP_Classes/Magnets/BP_MagnetBase.BP_MagnetBase_C|GetSphere _asbp_magnet_base) (* (Math|Vector|Normalize (- (Physics|GetCenterOfMass (LocalVariables|GetL_Pole) "None") (Physics|GetCenterOfMass (LocalVariables|GetL_Foreign_Pole) "None"))) (* (Math|Float|Square (/ (- _maxattractforce (Math|Float|Clamp(Float) (Math|Vector|VectorLength (- (Physics|GetCenterOfMass (LocalVariables|GetL_Pole) "None") (Physics|GetCenterOfMass (LocalVariables|GetL_Foreign_Pole) "None"))) 0.0 _maxattractforce)) _maxattractforce)) _maxattractforce)) "None" false))))
              (:2
                ;[1 1 1] South is Bix box
                (switch int _emovabletype
                  (:0
                    (Physics|AddForce (Variables|/Game/BP_Classes/Magnets/BP_MagnetBase.BP_MagnetBase_C|GetSphere _asbp_magnet_base) (* (Math|Vector|Normalize (- (Physics|GetCenterOfMass (LocalVariables|GetL_Pole) "None") (Physics|GetCenterOfMass (LocalVariables|GetL_Foreign_Pole) "None"))) (* (Math|Float|Square (/ (- _maxattractforce (Math|Float|Clamp(Float) (Math|Vector|VectorLength (- (Physics|GetCenterOfMass (LocalVariables|GetL_Pole) "None") (Physics|GetCenterOfMass (LocalVariables|GetL_Foreign_Pole) "None"))) 0.0 _maxattractforce)) _maxattractforce)) _maxattractforce)) "None" false))
                  (:1
                    (Physics|AddForce (Variables|Default|GetSphere) (* (* (Math|Vector|Normalize (- (Physics|GetCenterOfMass (LocalVariables|GetL_Pole) "None") (Physics|GetCenterOfMass (LocalVariables|GetL_Foreign_Pole) "None"))) (* (Math|Float|Square (/ (- _maxattractforce (Math|Float|Clamp(Float) (Math|Vector|VectorLength (- (Physics|GetCenterOfMass (LocalVariables|GetL_Pole) "None") (Physics|GetCenterOfMass (LocalVariables|GetL_Foreign_Pole) "None"))) 0.0 _maxattractforce)) _maxattractforce)) _maxattractforce)) -1.0) "None" false :!label _label_2))
                  (:2
                    (Physics|AddForce (Variables|/Game/BP_Classes/Magnets/BP_MagnetBase.BP_MagnetBase_C|GetSphere _asbp_magnet_base) (* (Math|Vector|Normalize (- (Physics|GetCenterOfMass (LocalVariables|GetL_Pole) "None") (Physics|GetCenterOfMass (LocalVariables|GetL_Foreign_Pole) "None"))) (* (Math|Float|Square (/ (- _maxattractforce (Math|Float|Clamp(Float) (Math|Vector|VectorLength (- (Physics|GetCenterOfMass (LocalVariables|GetL_Pole) "None") (Physics|GetCenterOfMass (LocalVariables|GetL_Foreign_Pole) "None"))) 0.0 _maxattractforce)) _maxattractforce)) _maxattractforce)) "None" false)
                    (goto _label_2)))))))))))