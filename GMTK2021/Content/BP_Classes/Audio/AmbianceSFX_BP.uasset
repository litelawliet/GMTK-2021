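; Ambiance audio actor that layers musical, diegetic and cave sound effects over a base ambiance.
; When AmbianceOn is set at BeginPlay, it fades in the base, then starts the three layers in staggered random delays.
; Each layer replays itself from OnAudioFinished after a random pause.
; IsMusicPlaying gates musical and cave plays and AmbianceOn gates diegetic; a blocked play ends that loop, as nothing here retries it.
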(event OnAudioFinished(MusicalSFX)
  ;[1 1 1] MusicalSFX
  (Utilities|FlowControl|Delay (Math|Random|RandomFloatinRange 0.0 1e+01))
  (CallFunction|PlayMusicalSFX))

(event OnAudioFinished(DiegeticSFX)
  ;[1 1 1] Diegetic
  (Utilities|FlowControl|Delay (Math|Random|RandomFloatinRange 1e+01 3e+01))
  (CallFunction|PlayDiegeticSFX))

(event OnAudioFinished(CaveSFX)
  ;[1 1 1] Cave
  (Utilities|FlowControl|Delay (Math|Random|RandomFloatinRange 1e+01 3e+01))
  (CallFunction|PlayCaveSFX))

(event EventBeginPlay
  ;[1 1 1] Ambiance Base
  (if (Variables|Default|GetAmbianceOn)
    (Audio|Components|Audio|FadeIn (Variables|Default|GetAmbianceBase) 4.0 1.0 0.0 "Linear" :!class /Script/Engine.AudioComponent)
    (Utilities|FlowControl|Delay (Math|Random|RandomFloatinRange 3.0 5.0))
    (CallFunction|PlayMusicalSFX)
    (Utilities|FlowControl|Delay (Math|Random|RandomFloatinRange 3.0 5.0))
    (CallFunction|PlayDiegeticSFX)
    (Utilities|FlowControl|Delay (Math|Random|RandomFloatinRange 1e+01 3e+01))
    (CallFunction|PlayCaveSFX)))

(event Collision|EventActorBeginOverlap
  (params (OtherActor :type Actor%20Object%20Reference)))

(fn ConstructionScript)

(fn PlayMusicalSFX
  (if (not (Variables|Default|GetIsMusicPlaying))
    (Audio|Components|Audio|Play (Variables|Default|GetMusicalSFX) 0.0)))

(fn PlayDiegeticSFX
  ;[1 1 1] Diegetic SFX
  (if (Variables|Default|GetAmbianceOn)
    (Audio|Components|Audio|Play (Variables|Default|GetDiegeticSFX) 0.0)))

(fn PlayCaveSFX
  (if (not (Variables|Default|GetIsMusicPlaying))
    (Audio|Components|Audio|Play (Variables|Default|GetCaveSFX) 0.0)))